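; Player controller that handles movement and camera-look axis input for the player character.
; BeginPlay caches the character, its capsule and, through a cast to BP_CharacterThirdPerson, its spring arm, which is not used further here.
; Forward/back and left/right axes move the character along the capsule's forward and right vectors rather than control rotation.
; Camera axes feed controller pitch and yaw input.
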(event `self.ReceiveBeginPlay`
  (bind _output_get (set `self.PlayerCharacter` (`GameplayStatics.GetPlayerCharacter` 0)))
  (set `self.PlayerCharacterCapsule` (`Character.CapsuleComponent` _output_get))
  (bind _asbp_character_third_person (cast `/Game/Player/BP_CharacterThirdPerson` (`self.PlayerCharacter`)))
  (set `self.Spring Arm` (`/Game/Player/BP_CharacterThirdPerson.SpringArm` _asbp_character_third_person)))

(event `InputAxis|Camera Rotate Yxis`
  (params (AxisValue :type "Float (single-precision)"))
  (`self.AddPitchInput` AxisValue))

(event `InputAxis|Forward/Back`
  (params (AxisValue :type "Float (single-precision)"))
  ;[1 1 1] Movement Player
  (`Pawn.AddMovementInput` (`self.PlayerCharacter`) (`SceneComponent.GetForwardVector` (`self.PlayerCharacterCapsule`)) AxisValue false))

(event `InputAxis|Camera Rotate Zxis`
  (params (AxisValue :type "Float (single-precision)"))
  (`self.AddYawInput` AxisValue))

(event `InputAxis|Left/Right` :consume false
  (params (AxisValue :type "Float (single-precision)"))
  ;[1 1 1] Movement Player
  (`Pawn.AddMovementInput` (`self.PlayerCharacter`) (`SceneComponent.GetRightVector` (`self.PlayerCharacterCapsule`)) AxisValue false))

(fn `UserConstructionScript`)