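; BP_SpawnEnemy is a spawner that populates an area with a randomized group of enemies when play begins.
; BeginPlay runs two random-length loops, one for TargetEnemy and one for PurifierEnemy, each calling SpawnEnemy.
; SpawnEnemy creates the AI pawn with the shared BT_Enemy behavior tree at a random point inside the SpawnLocation box.
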(event `self.ReceiveBeginPlay`
  (for _ (range (+ (`KismetMathLibrary.RandomIntegerInRange` 4 6) 1))
    (`self.SpawnEnemy` (`self.TargetEnemy`)))
  (for _ (range (+ (`KismetMathLibrary.RandomIntegerInRange` 2 4) 1))
    (`self.SpawnEnemy` (`self.PurifierEnemy`))))

(fn `SpawnEnemy`
  (params (Enemy :type "Pawn Class Reference"))
  (bind _spawnlocation (`self.SpawnLocation`))
  (`AIBlueprintHelperLibrary.SpawnAIFromClass` Enemy "/Game/Enemies/MovementEnemy/BT_Enemy.BT_Enemy" (`KismetMathLibrary.RandomPointInBoundingBox` (`SceneComponent.K2_GetComponentLocation` _spawnlocation) (`BoxComponent.GetScaledBoxExtent` _spawnlocation)) (struct) false null))

(fn `UserConstructionScript`)