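; BP_PurifierEnemy is an eraser enemy that the player paints on contact and that other unpainted purifiers can clean.
; When the third-person character overlaps its painting box, it swaps to the painted material, plays scribble effects and sets Painted.
; Overlapping an unpainted purifier restores a painted one's clean material.
; Each state change calls the interface's game stats and sends a plus or minus one enemy update.
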(event `self.BoxCollisionPainting.OnComponentBeginOverlap`
  (params (OverlappedComponent :type "PrimitiveComponent Object Reference") (OtherActor :type "Actor Object Reference") (OtherComp :type "PrimitiveComponent Object Reference") (OtherBodyIndex :type Integer) (bFromSweep :type Boolean) (SweepResult :type "HitResult Structure (by ref)"))
  (set `self.ActorBeginOverlapBoxCollision` OtherActor)
  (bind _asbp_purifier_enemy (cast `/Game/Enemies/BP_PurifierEnemy` (`self.ActorBeginOverlapBoxCollision`))
    (:`then`
      (if (`/Game/Enemies/BP_MasterEnemy.Painted` _asbp_purifier_enemy)
        _
        (elif (`self.Painted`)
          (`PrimitiveComponent.SetMaterial` (`self.eraser`) 0 "/Game/Enemies/StaticMeshes/Eraser/Т_Eraser.Т_Eraser")
          (set `self.Painted` false)
          (`/Game/Interface/W_InGame.GameStats` (`self.Interface`))
          (`self.SendNewDataOnEnemy` -1))))
    (:`CastFailed`
      (cast `/Game/Player/BP_CharacterThirdPerson` (`self.ActorBeginOverlapBoxCollision`))
      (if (not (`self.Painted`))
        (`PrimitiveComponent.SetMaterial` (`self.eraser`) 0 "/Game/Enemies/StaticMeshes/Eraser/Т_EraserPainted_.Т_EraserPainted_")
        (`NiagaraFunctionLibrary.SpawnSystemAttached` "/Game/Enemies/VFX/Scribble/NS_Scribble.NS_Scribble" (`self.CapsuleComponent`) "None" (0.0 0.0 0.0) (struct) "KeepRelativeOffset")
        (`GameplayStatics.PlaySound2D` "/Game/Music/Scribble.Scribble" 1.0 1.0 0.0 null null)
        (set `self.Painted` true)
        (`/Game/Interface/W_InGame.GameStats` (`self.Interface`))
        (`self.SendNewDataOnEnemy` 1)))))

(fn `UserConstructionScript`
  (`parent.UserConstructionScript`))