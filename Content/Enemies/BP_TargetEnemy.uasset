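; BP_TargetEnemy is a book enemy that can be painted, spreading its Painted state to others through contact.
; Overlaps on its painting box paint it when touched by the player or a painted target or purifier enemy, while an unpainted purifier cleans it.
; Painting swaps the book material and plays scribble VFX and sound; both changes report +1 or -1 through SendNewDataOnEnemy, and enemy-triggered ones also call CallGameStats.
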(event `self.BoxCollisionPainting.OnComponentBeginOverlap`
  (params (OverlappedComponent :type "PrimitiveComponent Object Reference") (OtherActor :type "Actor Object Reference") (OtherComp :type "PrimitiveComponent Object Reference") (OtherBodyIndex :type Integer) (bFromSweep :type Boolean) (SweepResult :type "HitResult Structure (by ref)"))
  (set `self.ActorOverlapBoxCollision` OtherActor)
  (`|ExecutionSequence`
    (:`then_0`
      (bind _asbp_target_enemy (cast `/Game/Enemies/BP_TargetEnemy` (`self.ActorOverlapBoxCollision`)))
      (if (`/Game/Enemies/BP_MasterEnemy.Painted` _asbp_target_enemy)
        (if (not (`self.Painted`))
          (`PrimitiveComponent.SetMaterial` (`self.Book`) 0 "/Game/Enemies/StaticMeshes/Book/GreenBookPainted/MI_Green_Book_vdkvbb2_2K_2.MI_Green_Book_vdkvbb2_2K_2")
          (`NiagaraFunctionLibrary.SpawnSystemAttached` "/Game/Enemies/VFX/Scribble/NS_Scribble.NS_Scribble" (`self.CapsuleComponent`) "None" (0.0 0.0 0.0) (struct) "KeepRelativeOffset" true)
          (`GameplayStatics.PlaySound2D` "/Game/Music/Scribble.Scribble" 1.0 1.0 0.0 null null)
          (set `self.Painted` true)
          (`/Game/Interface/W_InGame.GameStats` (`self.Interface`))
          (`self.SendNewDataOnEnemy` 1))))
    (:`then_1`
      (bind _asbp_purifier_enemy (cast `/Game/Enemies/BP_PurifierEnemy` (`self.ActorOverlapBoxCollision`)))
      (if (`/Game/Enemies/BP_MasterEnemy.Painted` _asbp_purifier_enemy)
        (if (not (`self.Painted`))
          (`PrimitiveComponent.SetMaterial` (`self.Book`) 0 "/Game/Enemies/StaticMeshes/Book/GreenBookPainted/MI_Green_Book_vdkvbb2_2K_2.MI_Green_Book_vdkvbb2_2K_2")
          (`NiagaraFunctionLibrary.SpawnSystemAttached` "/Game/Enemies/VFX/Scribble/NS_Scribble.NS_Scribble" (`self.CapsuleComponent`) "None" (0.0 0.0 0.0) (struct) "KeepRelativeOffset" true)
          (`GameplayStatics.PlaySound2D` "/Game/Music/Scribble.Scribble" 1.0 1.0 0.0 null null)
          (set `self.Painted` true)
          (`/Game/Interface/W_InGame.GameStats` (`self.Interface`))
          (`self.SendNewDataOnEnemy` 1))
        (elif (`self.Painted`)
          (`PrimitiveComponent.SetMaterial` (`self.Book`) 0 "/Game/Enemies/StaticMeshes/Book/GreenBookClear/MI_Green_Book_vdkvbb2_2K.MI_Green_Book_vdkvbb2_2K")
          (set `self.Painted` false)
          (`/Game/Interface/W_InGame.GameStats` (`self.Interface`))
          (`self.SendNewDataOnEnemy` -1))))
    (:`then_2`
      (cast `/Game/Player/BP_CharacterThirdPerson` (`self.ActorOverlapBoxCollision`))
      (if (not (`self.Painted`))
        (`PrimitiveComponent.SetMaterial` (`self.Book`) 0 "/Game/Enemies/StaticMeshes/Book/GreenBookPainted/MI_Green_Book_vdkvbb2_2K_2.MI_Green_Book_vdkvbb2_2K_2")
        (`NiagaraFunctionLibrary.SpawnSystemAttached` "/Game/Enemies/VFX/Scribble/NS_Scribble.NS_Scribble" (`self.CapsuleComponent`) "None" (0.0 0.0 0.0) (struct) "KeepRelativeOffset" true)
        (`GameplayStatics.PlaySound2D` "/Game/Music/Scribble.Scribble" 1.0 1.0 0.0 null null)
        (set `self.Painted` true)
        (`self.SendNewDataOnEnemy` 1)))))

(fn `UserConstructionScript`
  (`parent.UserConstructionScript`))