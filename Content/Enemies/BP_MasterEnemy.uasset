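; BP_MasterEnemy is an enemy Blueprint, apparently a base class, that feeds painted-enemy progress to the third-person player character.
; After a brief BeginPlay delay, each instance caches the player and its Interface, counts all enemies, and resets the painted count.
; SendNewDataOnEnemy adjusts the player's painted count by a given delta against that cached total.
; The player overlapping BoxCollisionPainting triggers CallGameStats on the Interface.
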(event `self.ReceiveBeginPlay`
  (`KismetSystemLibrary.Delay` 0.01)
  (bind _asbp_character_third_person (cast `/Game/Player/BP_CharacterThirdPerson` (`GameplayStatics.GetPlayerCharacter` 0)))
  (set `self.As BP Character Third Person` _asbp_character_third_person)
  (set `self.Interface` (`/Game/Player/BP_CharacterThirdPerson.Interface` _asbp_character_third_person))
  (bind _outactors (`GameplayStatics.GetAllActorsOfClass` "BP_MasterEnemy_C"))
  (bind _returnvalue (`KismetArrayLibrary.Array_Length` _outactors))
  (set `self.AllTargetEnemy` _returnvalue)
  (`/Game/Player/BP_CharacterThirdPerson.CheckPaintedEnemy` (`self.As BP Character Third Person`) 0 _returnvalue))

(event `self.BoxCollisionPainting.OnComponentBeginOverlap`
  (params (OverlappedComponent :type "PrimitiveComponent Object Reference") (OtherActor :type "Actor Object Reference") (OtherComp :type "PrimitiveComponent Object Reference") (OtherBodyIndex :type Integer) (bFromSweep :type Boolean) (SweepResult :type "HitResult Structure (by ref)"))
  (cast `/Game/Player/BP_CharacterThirdPerson` OtherActor)
  (`/Game/Interface/W_InGame.GameStats` (`self.Interface`)))

(fn `SendNewDataOnEnemy`
  (params (`Add/Sub` :type Integer))
  (`/Game/Player/BP_CharacterThirdPerson.CheckPaintedEnemy` (`self.As BP Character Third Person`) (+ (`/Game/Player/BP_CharacterThirdPerson.PaintedEnemy` (`self.As BP Character Third Person`)) `Add/Sub`) (`self.AllTargetEnemy`)))

(fn `UserConstructionScript`)